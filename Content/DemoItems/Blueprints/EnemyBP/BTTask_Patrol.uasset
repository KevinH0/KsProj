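; Behavior tree task for enemy AI patrols, built around a map of waypoint actors to wait times.
; On execute it copies PatrolPath from the pawn's BP_EnemyBehavior component, failing if missing or empty, with no call into the movement loop.
; The loop moves to each waypoint, waits its mapped time on a timer, then wraps around indefinitely, failing only when a move fails.
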(event Custom|moveToPatrol
  (bind _patrolpath (Variables|Default|GetPatrolPath))
  (bind _keys (Utilities|Map|Keys (Variables|Default|GetPatrolPath)))
  (AI|AIMoveTo (Variables|Default|GetControlled%20Pawn) (Transformation|GetActorLocation (Utilities|Array|Get(acopy) _keys (Variables|Default|GetPatrolIndex))) 0 5.0 false
    (:OnSuccess
      (bind _keys_2 (Utilities|Map|Keys _patrolpath))
      (Utilities|Time|SetTimerbyEvent (delegate Custom|endWait) (.Value (Utilities|Map|Find _patrolpath (Utilities|Array|Get(acopy) _keys_2 (Variables|Default|GetPatrolIndex))))))
    (:OnFail
      (AI|BehaviorTree|FinishExecute false))))

(event Custom|endWait
  (bind _result (Math|Integer|IncrementInt (Variables|Default|GetPatrolIndex))
    (:%20%20
      (if (>= _result (Utilities|Map|Length (Variables|Default|GetPatrolPath)))
        (Variables|Default|SetPatrolIndex 0)
        (CallFunction|MovetoPatrol)
        (else
          (CallFunction|MovetoPatrol))))))

(event EventReceiveExecuteAI
  (params (OwnerController :type AI%20Controller%20Object%20Reference) (ControlledPawn :type Pawn%20Object%20Reference))
  (bind _returnvalue (Actor|GetComponentbyClass ControlledPawn "/Game/DemoItems/Blueprints/EnemyBP/BP_EnemyBehavior.BP_EnemyBehavior_C"))
  (bind _patrolpath (Variables|/Game/DemoItems/Blueprints/EnemyBP/BP_EnemyBehavior.BP_EnemyBehavior_C|GetpatrolPath _returnvalue))
  (Variables|Default|SetControlled%20Pawn ControlledPawn)
  (Utilities|IsValid _returnvalue
    (:Is%20Valid
      (if (> (Utilities|Map|Length _patrolpath) 0)
        (Variables|Default|SetPatrolPath _patrolpath)
        (else
          (AI|BehaviorTree|FinishExecute false))))
    (:Is%20Not%20Valid
      (AI|BehaviorTree|FinishExecute false))))