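; RunnerEnemy is an enemy character that chases the player once it sees a pawn or hears noise, and dies from damage.
; PawnSensing events latch LocatePlayer and trigger an AI MoveTo toward the player; until then, Tick keeps stopping its movement.
; On reaching range it plays a slowed rifle montage, using InAtkRange and a montage-length delay to gate replays.
; AnyDamage reduces EnemyHealth and destroys the actor at zero.
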(event OnSeePawn(PawnSensing)
  (params (Pawn :type Pawn%20Object%20Reference))
  (if true
    (Variables|Default|SetlocatePlayer true)
    (CallFunction|FollowPlayer)
    (else
      (Variables|Default|SetinAtkRange false))))

(event OnHearNoise(PawnSensing)
  (params (Instigator :type Pawn%20Object%20Reference) (Location :type Vector%20%28by%20ref%29 :default "0, 0, 0") (Volume :type Float%20%28single-precision%29))
  (Variables|Default|SetlocatePlayer true)
  (CallFunction|FollowPlayer))

(event Custom|FollowPlayer
  (Variables|Default|SetinAtkRange true)
  (if (Variables|Default|GetlocatePlayer)
    (AI|AIMoveTo self "0, 0, 0" (Game|GetPlayerCharacter 0) 2.5e+02 false
      (:OnSuccess
        (if (Variables|Default|GetinAtkRange)
          (Variables|Default|SetinAtkRange false)
          (bind _returnvalue (Animation|PlayAnimMontage "/Game/DemoItems/Animation/EnemyRifleMontage.EnemyRifleMontage" 0.4 "None"))
          (Utilities|FlowControl|Delay _returnvalue)
          (Variables|Default|SetinAtkRange true))))))

(event EventBeginPlay)

(event Collision|EventActorBeginOverlap
  (params (OtherActor :type Actor%20Object%20Reference)))

(event EventTick
  (params (DeltaSeconds :type Float%20%28single-precision%29))
  (if (not (Variables|Default|GetlocatePlayer))
    (Class|NavMovementComponent|StopMovementKeepPathing (Variables|Character|GetCharacterMovement))))

(event Game|Damage|EventAnyDamage
  (params (Damage :type Float%20%28single-precision%29) (DamageType :type Damage%20Type%20Object%20Reference) (InstigatedBy :type Controller%20Object%20Reference) (DamageCauser :type Actor%20Object%20Reference))
  (bind _output_get (Variables|Default|SetEnemyHealth (- (Variables|Default|GetEnemyHealth) Damage)))
  (if (<= _output_get 0.0)
    (Actor|DestroyActor)))

(fn ConstructionScript)