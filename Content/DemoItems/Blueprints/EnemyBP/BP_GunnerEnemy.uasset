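; Rifle-wielding AI enemy that wanders, pursues the player and fires bullets with random spread.
; Pawn sensing triggers a move toward the player and alternating fire and cooldown, though its sighting flags reset in the same sequence.
; Player damage, reduced by armor and multiplied on crits, lowers health and updates the enemy widget.
; Only the non-crit branch checks for death, which increments player score and destroys the actor.
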(event OnSeePawn(PawnSensing)
  (params (Pawn :type Pawn%20Object%20Reference))
  (bind _bullet_spawn (Variables|Default|GetBullet%20spawn))
  (bind _returnvalue (Transformation|GetWorldRotation _bullet_spawn))
  (bind _asbp_first_person_character (Utilities|Casting|CastToBP_FirstPersonCharacter Pawn))
  (Utilities|FlowControl|Sequence
    (:then_0
      (Variables|Default|SetlocatePlayer true)
      (Variables|Default|SettargetedPlayer true)
      (AI|AIMoveTo self "0, 0, 0" _asbp_first_person_character 2.5e+02 false
        (:then
          (if (Variables|Default|GetcanAtk)
            (Transformation|SetActorRotation (Math|Rotator|FindRelativeLookatRotation (Math|Conversions|ToTransform(Vector) (Transformation|GetActorLocation)) (Transformation|GetActorLocation _asbp_first_person_character)))
            (Variables|Default|SetcanAtk (Variables|Default|GetcanAtk))
            (Components|Movement|StopMovementImmediately (Variables|Character|GetCharacterMovement))
            (Game|SpawnActorfromClass "/Game/DemoItems/Blueprints/BulletBP/BP_RifleBullet.BP_RifleBullet_C" (Math|Transform|MakeTransform (Transformation|GetWorldLocation _bullet_spawn) (Math|Rotator|MakeRotator (.roll _returnvalue) (+ (Math|Random|RandomFloatinRange -5.0 5.0) (.pitch _returnvalue)) (+ (.yaw _returnvalue) (Math|Random|RandomFloatinRange -5.0 5.0)))) "Undefined" "MultiplyWithRoot" 0 0)
            (bind _returnvalue_2 (Animation|PlayAnimMontage "/Game/DemoItems/Animation/EnemyRifleMontage.EnemyRifleMontage" 0.7 "None"))
            (Utilities|FlowControl|Delay _returnvalue_2)
            (Variables|Default|SetcanAtk false)
            (else
              (Utilities|FlowControl|Delay (Variables|Default|GetatkRate))
              (Variables|Default|SetcanAtk true))))))
    (:then_1
      (Variables|Default|SetlocatePlayer false)
      (Variables|Default|SettargetedPlayer false))))

(event Custom|LocateFollowPlayer
  (if (not (Variables|Default|GetlocatePlayer))
    (AI|AIMoveTo self "0, 0, 0" (Game|GetPlayerCharacter 0) 2.5e+02 false)))

(event EventBeginPlay
  (Variables|Default|SetcurrentHp (Variables|Default|GetmaxHp))
  (CallFunction|LocateFollowPlayer)
  (Transformation|AttachComponentToComponent (Variables|Default|Getfinal) (Variables|Character|GetMesh) "thumb_01_l" "KeepRelative" "KeepRelative" "KeepRelative" true))

(event EventTick
  (params (DeltaSeconds :type Float%20%28single-precision%29))
  (if (not (Variables|Default|GetlocatePlayer))
    (Utilities|FlowControl|Delay (Math|Random|RandomFloatinRange 2.0 3.0))
    (AI|AIMoveTo self (.RandomLocation (AI|Navigation|GetRandomReachablePointinRadius (Transformation|GetActorLocation) 1e+03 0 0)) 0 5.0 false)))

(event Game|Damage|EventAnyDamage
  (params (Damage :type Float%20%28single-precision%29) (DamageType :type Damage%20Type%20Object%20Reference) (InstigatedBy :type Controller%20Object%20Reference) (DamageCauser :type Actor%20Object%20Reference))
  (bind _critmulti (Variables|Default|GetCritMulti))
  (bind _armor (Variables|Default|GetArmor))
  (bind _returnvalue (- Damage _armor))
  (bind _returnvalue_2 (* _returnvalue _critmulti))
  (if (Variables|Default|GetonCrit)
    (Utilities|Casting|CastToPlayerDamageType DamageType)
    (Variables|Default|SetcurrentHp (Math|Float|Clamp(Float) (- (Variables|Default|GetcurrentHp) _returnvalue_2) 0.0 (Variables|Default|GetmaxHp)))
    (bind _asenemy_widget (Utilities|Casting|CastToEnemyWidget (UserInterface|GetWidget (Variables|Default|GetDamage))))
    (Default|DamageUI _asenemy_widget true _returnvalue_2 0.0)
    (else
      (Utilities|Casting|CastToPlayerDamageType DamageType)
      (Variables|Default|SetcurrentHp (Math|Float|Clamp(Float) (- (Variables|Default|GetcurrentHp) _returnvalue) 0.0 (Variables|Default|GetmaxHp)))
      (bind _asenemy_widget_2 (Utilities|Casting|CastToEnemyWidget (UserInterface|GetWidget (Variables|Default|GetDamage))))
      (Default|DamageUI _asenemy_widget_2 false 0.0 _returnvalue)
      (if (== (Variables|Default|GetcurrentHp) 0.0)
        (bind _output_get (Variables|Default|SetAs%20BP%20First%20Person%20Character (stale OnSeePawn(PawnSensing) _asbp_first_person_character)))
        (bind _result (Math|Integer|IncrementInt (Variables|/Game/DemoItems/Blueprints/Player/BP_FirstPersonCharacter.BP_FirstPersonCharacter_C|Getscore _output_get))
          (:%20%20
            (Variables|/Game/DemoItems/Blueprints/Player/BP_FirstPersonCharacter.BP_FirstPersonCharacter_C|Setscore _output_get _result)
            (Actor|DestroyActor)))))))

(fn ConstructionScript)