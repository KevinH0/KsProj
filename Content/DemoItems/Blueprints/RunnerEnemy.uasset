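; RunnerEnemy is an AI character Blueprint that chases the player once it sees or hears a pawn, then plays an attack montage.
; PawnSensing events set LocatePlayer and trigger an AI move toward the player character, while Tick halts movement until LocatePlayer is set.
; On arrival it plays the rifle montage if InAtkRange is true, clearing that flag; nothing here sets it again or resets LocatePlayer.
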(event OnSeePawn(PawnSensing)
  (params (Pawn :type Pawn%20Object%20Reference))
  (Variables|Default|SetlocatePlayer true)
  (CallFunction|FollowPlayer))

(event OnHearNoise(PawnSensing)
  (params (Instigator :type Pawn%20Object%20Reference) (Location :type Vector%20%28by%20ref%29 :default "0, 0, 0") (Volume :type Float%20%28single-precision%29))
  (Variables|Default|SetlocatePlayer true)
  (CallFunction|FollowPlayer))

(event Custom|FollowPlayer
  (if (Variables|Default|GetlocatePlayer)
    (AI|AIMoveTo self "0, 0, 0" (Game|GetPlayerCharacter 0) 2.5e+02 false
      (:OnSuccess
        (if (Variables|Default|GetinAtkRange)
          (Variables|Default|SetinAtkRange false)
          (Animation|PlayAnimMontage "/Game/DemoItems/AnimationBP/EnemyRifleMontage.EnemyRifleMontage" 1.0 "None"))))))

(event EventBeginPlay)

(event Collision|EventActorBeginOverlap
  (params (OtherActor :type Actor%20Object%20Reference)))

(event EventTick
  (params (DeltaSeconds :type Float%20%28single-precision%29))
  (if (not (Variables|Default|GetlocatePlayer))
    (Class|NavMovementComponent|StopMovementKeepPathing (Variables|Character|GetCharacterMovement))))

(fn ConstructionScript)