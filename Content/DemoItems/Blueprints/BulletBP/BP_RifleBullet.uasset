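; BP_RifleBullet is a rifle projectile that pushes physics objects and damages the first-person player character.
; On hit, it applies an impulse scaled from its velocity to any physics-simulating component, and is destroyed whatever it hit.
; On overlap with a BP_FirstPersonCharacter, it applies a small fixed PlayerDamageType damage and destroys itself.
; Overlaps with other actors fail the cast and leave the bullet alive.
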(event Collision|EventActorBeginOverlap
  (params (OtherActor :type Actor%20Object%20Reference))
  (bind _asbp_first_person_character (Utilities|Casting|CastToBP_FirstPersonCharacter OtherActor))
  (Utilities|IsValid _asbp_first_person_character
    (:Is%20Valid
      (Game|Damage|ApplyDamage _asbp_first_person_character 5.0 0 (Components|GetOwner (Variables|Default|GetStaticMesh)) "/Game/DemoItems/Blueprints/BulletBP/PlayerDamageType.PlayerDamageType_C")
      (Actor|DestroyActor))
    (:Is%20Not%20Valid
      (Actor|DestroyActor))))

(event Collision|EventHit
  (params (MyComp :type Primitive%20Component%20Object%20Reference) (Other :type Actor%20Object%20Reference) (OtherComp :type Primitive%20Component%20Object%20Reference) (bSelfMoved :type Boolean) (HitLocation :type Vector :default "0, 0, 0") (HitNormal :type Vector :default "0, 0, 0") (NormalImpulse :type Vector :default "0, 0, 0") (Hit :type Hit%20Result%20Structure%20%28by%20ref%29))
  (if (Physics|IsSimulatingPhysics OtherComp "None")
    (Physics|AddImpulseatLocation OtherComp (* (Transformation|GetVelocity) 1e+02) (Transformation|GetActorLocation) "None")
    (Actor|DestroyActor)
    (else
      (Actor|DestroyActor))))

(fn ConstructionScript)