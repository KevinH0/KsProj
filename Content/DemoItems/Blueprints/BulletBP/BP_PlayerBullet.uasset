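; BP_PlayerBullet is the player's projectile, which damages gunner enemies it overlaps.
; An enemy overlap applies PlayerDamageType damage and destroys the bullet; other overlaps also destroy it, except the first-person character.
; A blocking hit on a physics-simulating component applies a velocity-based impulse and destroys the hit actor, otherwise the bullet destroys itself.
; A Delay on Tick caps its lifetime at a few seconds.
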(event EventTick
  (params (DeltaSeconds :type Float%20%28single-precision%29))
  (Utilities|FlowControl|Delay 5.0)
  (Actor|DestroyActor))

(event Collision|EventActorBeginOverlap
  (params (OtherActor :type Actor%20Object%20Reference))
  (bind _asbp_gunner_enemy (Utilities|Casting|CastToBP_GunnerEnemy OtherActor)
    (:then
      (Utilities|IsValid _asbp_gunner_enemy
        (:Is%20Valid
          (Game|Damage|ApplyDamage _asbp_gunner_enemy 4e+01 0 (Components|GetOwner (Variables|Default|GetSphere)) "/Game/DemoItems/Blueprints/BulletBP/PlayerDamageType.PlayerDamageType_C")
          (Actor|DestroyActor))
        (:Is%20Not%20Valid
          (Actor|DestroyActor))))
    (:CastFailed
      (Utilities|Casting|CastToBP_FirstPersonCharacter OtherActor
        (:CastFailed
          (Actor|DestroyActor))))))

(event Collision|EventHit
  (params (MyComp :type Primitive%20Component%20Object%20Reference) (Other :type Actor%20Object%20Reference) (OtherComp :type Primitive%20Component%20Object%20Reference) (bSelfMoved :type Boolean) (HitLocation :type Vector :default "0, 0, 0") (HitNormal :type Vector :default "0, 0, 0") (NormalImpulse :type Vector :default "0, 0, 0") (Hit :type Hit%20Result%20Structure%20%28by%20ref%29))
  (Development|PrintString "1")
  (if (Physics|IsSimulatingPhysics OtherComp "None")
    (Physics|AddImpulseatLocation OtherComp (* (Transformation|GetVelocity) 1e+02) (Transformation|GetActorLocation) "None")
    (Actor|DestroyActor Other)
    (else
      (Actor|DestroyActor))))

(fn ConstructionScript)